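; BP_Equipable is an equipable item actor that shows its name when the cursor hovers over it.
; The construction script sets the skeletal mesh from the Data variable's Mesh field.
; On BeginPlay, Data's Name is written into the WBP_ItemName widget held by the ItemNameWidget component.
; Cursor-over events on the skeletal mesh toggle that component's visibility.
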(event OnBeginCursorOver(SkeletalMesh)
  (params (TouchedComponent :type Primitive%20Component%20Object%20Reference))
  (CallFunction|ShowItemNameonScreen))

(event OnEndCursorOver(SkeletalMesh)
  (params (TouchedComponent :type Primitive%20Component%20Object%20Reference))
  (CallFunction|HideItemNameonScreen))

(event EventBeginPlay
  (CallFunction|SetTexttoItemTextWidget (.Name (Utilities|Struct|BreakS_ItemData (Variables|Default|GetData)))))

(fn ConstructionScript
  (CallFunction|UpdateMesh))

(fn ShowItemNameonScreen
  (Rendering|SetVisibility (Variables|Default|GetItemNameWidget) true false))

(fn HideItemNameonScreen
  (Rendering|SetVisibility (Variables|Default|GetItemNameWidget) false false))

(fn SetTexttoItemTextWidget
  (params (Text :type Name))
  (bind _aswbp_item_name (Utilities|Casting|CastToWBP_ItemName (UserInterface|GetUserWidgetObject (Variables|Default|GetItemNameWidget)))
    (:then
      _)
    (:CastFailed
      _))
  (Rendering|Components|TextRender|SetText (Variables|/Game/UMG/WBP_ItemName.WBP_ItemName_C|GetItemNameText _aswbp_item_name) (Utilities|Text|ToText(Name) Text)))

(fn UpdateMesh
  (Class|SkinnedMeshComponent|SetSkeletalMesh (Variables|Default|GetSkeletalMesh) (.Mesh (Utilities|Struct|BreakS_ItemData (Variables|Default|GetData))) false))