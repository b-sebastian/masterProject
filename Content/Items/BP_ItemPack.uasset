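; BP_ItemPack is a world item that shows its name in a widget when the cursor hovers over its skeletal mesh.
; BeginPlay writes Data.Name into the WBP_ItemName widget, and cursor begin/end events toggle that widget's visibility.
; RandomizeData, not called within this Blueprint, uses nested random switches to fill the item struct as a weapon, armor piece or potion with rolled stats.
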(event OnBeginCursorOver(SkeletalMesh)
  (params (TouchedComponent :type Primitive%20Component%20Object%20Reference))
  (CallFunction|ShowItemNameonScreen))

(event OnEndCursorOver(SkeletalMesh)
  (params (TouchedComponent :type Primitive%20Component%20Object%20Reference))
  (CallFunction|HideItemNameonScreen))

(event EventBeginPlay
  (CallFunction|SetTexttoItemTextWidget (.Name (Utilities|Struct|BreakS_ItemData (Variables|Default|GetData)))))

(fn ConstructionScript)

(fn ShowItemNameonScreen
  (Rendering|SetVisibility (Variables|Default|GetItemNameWidget) true false))

(fn HideItemNameonScreen
  (Rendering|SetVisibility (Variables|Default|GetItemNameWidget) false false))

(fn SetTexttoItemTextWidget
  (params (Text :type Name))
  (bind _aswbp_item_name (Utilities|Casting|CastToWBP_ItemName (UserInterface|GetUserWidgetObject (Variables|Default|GetItemNameWidget)))
    (:then
      _)
    (:CastFailed
      _))
  (Rendering|Components|TextRender|SetText (Variables|/Game/UMG/WBP_ItemName.WBP_ItemName_C|GetItemNameText _aswbp_item_name) (Utilities|Text|ToText(Name) Text)))

(fn RandomizeData
  (bind _returnvalue (Math|Random|RandomIntegerinRange 5 30))
  (bind _data (Variables|Default|GetData))
  (bind _returnvalue_2 (Math|Conversions|ToFloat(Integer) _returnvalue))
  (switch int (Math|Random|RandomIntegerinRange 0 1)
    (:0
      (Utilities|Struct|SetmembersinS_ItemData (Variables|Default|GetData) true)
      (switch int (Math|Random|RandomIntegerinRange 0 1)
        (:0
          ;[1 1 1] Weapon
          (Utilities|Struct|SetmembersinS_ItemData (Variables|Default|GetData) "NewEnumerator3")
          (switch int (Math|Random|RandomIntegerinRange 0 1)
            (:0
              (Utilities|Struct|SetmembersinS_ItemData (Variables|Default|GetData) "One Handed Sword" (Math|Conversions|ToFloat(Integer) (Math|Random|RandomIntegerinRange 10 50)) "/Game/InfinityBladeWeapons/Weapons/Blade/Swords/Blade_BlackWyrmBlade/T_Blade_BlackWyrmBlade1_D.T_Blade_BlackWyrmBlade1_D" "/Game/InfinityBladeWeapons/Weapons/Blade/Swords/Blade_BlackWyrmBlade/SK_Blade_BlackWyrmBlade.SK_Blade_BlackWyrmBlade"))
            (:1
              (Utilities|Struct|SetmembersinS_ItemData (Variables|Default|GetData) "Two Handed Great Sword" (Math|Conversions|ToFloat(Integer) (Math|Random|RandomIntegerinRange 20 100)) "/Game/InfinityBladeWeapons/Weapons/Blade/Axes/Blade_AnthraciteAxe/T_Blade_AnthraciteAxe1_D.T_Blade_AnthraciteAxe1_D" "/Game/InfinityBladeWeapons/Weapons/Blade/Silly_Weapons/Blade_Chainsaw/SK_Blade_Chainsaw.SK_Blade_Chainsaw"))))
        (:1
          ;[1 1 1] Clothing
          (switch int (Math|Random|RandomIntegerinRange 0 3)
            (:0
              (Utilities|Struct|SetmembersinS_ItemData _data "Helmet" _returnvalue_2 "/Game/Items/Clothing/Head/TN_Warrior_Head_Basic.TN_Warrior_Head_Basic" "NewEnumerator0" "/Game/Items/Clothing/Head/SM_Warrior_Head_Basic.SM_Warrior_Head_Basic"))
            (:1
              (Utilities|Struct|SetmembersinS_ItemData _data "Plate" _returnvalue_2 "/Game/Items/Clothing/Body/TN_Warrior_Body_Basic.TN_Warrior_Body_Basic" "NewEnumerator1" "/Game/Items/Clothing/Body/SM_Warrior_Body_Basic.SM_Warrior_Body_Basic"))
            (:2
              (Utilities|Struct|SetmembersinS_ItemData _data "Boots" _returnvalue_2 "/Game/InfinityBladeWeapons/Weapons/Blade/Swords/Blade_BlackKnight/T_Blade_BlackKnight_Sword1_D.T_Blade_BlackKnight_Sword1_D" "NewEnumerator2" "/Game/Items/Clothing/Feet/SM_Warrior_Feet_Basic.SM_Warrior_Feet_Basic"))
            (:3
              (Utilities|Struct|SetmembersinS_ItemData _data "Gloves" _returnvalue_2 "/Game/InfinityBladeWeapons/Weapons/Blade/Silly_Weapons/Blade_Bubblewand/T_Blade_Bubblewand2_N.T_Blade_Bubblewand2_N" "NewEnumerator4" "/Game/Items/Clothing/Hands/SM_Warrior_Hands_Basic.SM_Warrior_Hands_Basic"))))))
    (:1
      ;[1 1 1] Potion
      (Utilities|Struct|SetmembersinS_ItemData (Variables|Default|GetData) "Potion" (Math|Conversions|ToFloat(Integer) (Math|Random|RandomIntegerinRange 0 20)) (Math|Conversions|ToFloat(Integer) (Math|Random|RandomIntegerinRange 0 20)) "/Game/InfinityBladeWeapons/Weapons/Blade/Silly_Weapons/Blade_Balloon/T_Blade_Balloon1_D.T_Blade_Balloon1_D" true))))