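; Ally decoy that lures enemy AI with noise and disappears once a targeting enemy gets close.
; From BeginPlay, a looping Delay repeatedly plays an explosion sound and emits PawnMakeNoise at its location.
; A throttled Tick scans all BP_EnemyController targets for itself and compares capsule distance to that enemy character.
; Within range, it removes itself from that controller's Targets and destroys itself.
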(event EventBeginPlay
  ;[1 1 1] Play sound every 2sec
  (Audio|PlaySoundatLocation "/Game/StarterContent/Audio/Explosion01.Explosion01" (Transformation|GetActorLocation) :!label _label)
  (Class|Pawn|PawnMakeNoise 1.0 "0, 0, 0" true self)
  (Utilities|FlowControl|Delay 2.0)
  (goto _label))

(event EventTick
  (params (DeltaSeconds :type Float%20%28single-precision%29))
  ;[1 1 1] Destroy self actor if Enemy is close to it and sees it
  (bind _output_get (Variables|Default|SetRefreshCounter (+ DeltaSeconds (Variables|Default|GetRefreshCounter))))
  (if (>= _output_get 0.5)
    (Variables|Default|SetRefreshCounter 0.0)
    (bind _outactors (Actor|GetAllActorsOfClass "/Game/AI/Enemy/BP_EnemyController.BP_EnemyController_C"))
    (for _array_element _outactors
      (if (Utilities|Array|ContainsItem (Variables|/Game/AI/Enemy/BP_EnemyController.BP_EnemyController_C|GetTargets _array_element) self)
        (bind _asbp_enemy_character (Utilities|Casting|CastToBP_EnemyCharacter (Pawn|GetControlledPawn _array_element)))
        (if (<= (Math|Vector|VectorLength (- (Transformation|GetWorldLocation (Variables|Default|GetCapsuleComponent)) (Transformation|GetWorldLocation (Variables|/Script/Engine.Character|GetCapsuleComponent _asbp_enemy_character)))) 5e+02)
          (Utilities|Array|RemoveItem (Variables|/Game/AI/Enemy/BP_EnemyController.BP_EnemyController_C|GetTargets _array_element) self)
          (Actor|DestroyActor))))))

(fn ConstructionScript
  (|CallParentFunction))