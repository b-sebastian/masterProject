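; Enemy AI controller that starts the enemy behavior tree and blackboard on StartAI, then feeds it perception results.
; Perception tracks sensed ally characters, fills an empty Target key and, when the last is lost, clears the sensing flag and saves its position unless it is a decoy.
; For pawns using stamina, Tick drains it at high speed and zeroes walk speed on exhaustion until a delayed loop refills it.
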(event OnTargetPerceptionUpdated(AIPerception)
  (params (Actor :type Actor%20Object%20Reference) (Stimulus :type AI%20Stimulus%20Structure))
  (bind _returnvalue (AI|GetBlackboard 0))
  (bind _returnvalue_2 (Utilities|Name|MakeLiteralName "IsSensingAPlayer"))
  (bind _returnvalue_3 (Utilities|Name|MakeLiteralName "Target"))
  (bind _targets (Variables|Default|GetTargets))
  ;[1 1 1] Find targets
  (if (Variables|AI|GetIsAIActive)
    (bind _ascharacter (Utilities|Casting|CastToCharacter Actor))
    (Utilities|Casting|CastToBP_AllyCharacterBase _ascharacter)
    (if (.bSuccessfullySensed (Utilities|Struct|BreakAIStimulus Stimulus))
      (Utilities|Array|AddUnique _targets _ascharacter)
      (AI|Components|Blackboard|SetValueasBool _returnvalue _returnvalue_2 true)
      (if (== (AI|Components|Blackboard|GetValueasObject _returnvalue _returnvalue_3) 0)
        (AI|Components|Blackboard|SetValueasObject _returnvalue _returnvalue_3 _ascharacter))
      (else
        (Utilities|Array|RemoveItem _targets _ascharacter)
        (if (== (Utilities|Array|Length _targets) 0)
          (AI|Components|Blackboard|SetValueasBool _returnvalue _returnvalue_2 false)
          (Utilities|Casting|CastToBP_AllyDecoy _ascharacter
            (:CastFailed
              (AI|Components|Blackboard|SetValueasVector _returnvalue (Utilities|Name|MakeLiteralName "LastKnownPosition") (Transformation|GetActorLocation _ascharacter)))))))))

(event Custom|Start%20AI
  ;[1 1 1] Blackboard Initial setup for Enemy
  (Utilities|FlowControl|Sequence
    (:then_0
      (Class|AIController|UseBlackboard "/Game/AI/Enemy/BB_Enemy.BB_Enemy")
      (AI|RunBehaviorTree "/Game/AI/Enemy/BT_Enemy.BT_Enemy")
      (Variables|AI|SetIsAIActive true))))

(event EventTick
  (params (DeltaSeconds :type Float%20%28single-precision%29))
  ;[1 1 1] Stamina
  (if (Variables|/Game/AI/Enemy/BP_EnemyCharacter.BP_EnemyCharacter_C|GetuseStamina (Variables|Default|GetselfCharacter))
    (Utilities|FlowControl|Sequence
      (:then_0
        (if (<= (Variables|Default|GetStamina) 0.0)
          (Variables|Default|SetIsExhausted true)
          (Variables|Default|SetStamina (+ (Variables|Default|GetStamina) (/ (Variables|Default|GetMaxStamina) 1e+01)) :!label _label)
          (if (>= (Variables|Default|GetStamina) (Variables|Default|GetMaxStamina))
            (Variables|Default|SetStamina (Variables|Default|GetMaxStamina))
            (Variables|Default|SetIsExhausted false)
            (else
              (Utilities|FlowControl|Delay 0.2)
              (goto _label)))))
      (:then_1
        (bind _asbp_enemy_character (Utilities|Casting|CastToBP_EnemyCharacter (Pawn|GetControlledPawn)))
        (if (Variables|Default|GetIsExhausted)
          (Variables|/Script/Engine.CharacterMovementComponent|SetMaxWalkSpeed (Variables|/Script/Engine.Character|GetCharacterMovement _asbp_enemy_character) 0.0)
          (else
            (Variables|/Script/Engine.CharacterMovementComponent|SetMaxWalkSpeed (Variables|/Script/Engine.Character|GetCharacterMovement _asbp_enemy_character) (Variables|/Game/AI/Enemy/BP_EnemyCharacter.BP_EnemyCharacter_C|GetMax%20Walk%20Speed _asbp_enemy_character)))))
      (:then_2
        (bind _asbp_enemy_character_2 (Utilities|Casting|CastToBP_EnemyCharacter (Pawn|GetControlledPawn)))
        (if (>= (Math|Vector|VectorLength (Transformation|GetVelocity _asbp_enemy_character_2)) 5e+02)
          (Variables|Default|SetStamina (- (Variables|Default|GetStamina) (* DeltaSeconds 5e+01))))))))

(event EventBeginPlay
  (bind _asbp_enemy_character (Utilities|Casting|CastToBP_EnemyCharacter (Pawn|GetControlledPawn)))
  (Variables|Default|SetselfCharacter _asbp_enemy_character))

(fn ConstructionScript)