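; BP_EnemySpawn is a placed spawner actor that populates its area with BP_EnemyCharacter enemies when play begins.
; On BeginPlay it spawns a random count between its minimum and maximum variables, each at a random XY offset in a square around the actor with a random yaw.
; Spawns nudge to avoid collisions and are skipped if no clear spot is found, so fewer enemies can appear.
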(event EventBeginPlay
  (bind _self self)
  (bind _returnvalue (Transformation|GetActorTransform _self))
  (bind (_x _y _z) (Math|Vector|BreakVector (.location _returnvalue)))
  (for _index (range 1 (Math|Random|RandomIntegerinRange (Variables|Default|GetMinNumberOfEnemies) (Variables|Default|GetMaxNumberOfEnemies)))
    (Game|SpawnActorfromClass "/Game/AI/Enemy/BP_EnemyCharacter.BP_EnemyCharacter_C" (Math|Transform|MakeTransform (Math|Vector|MakeVector (+ (Math|Random|RandomFloatinRange -2e+02 2e+02) _x) (+ _y (Math|Random|RandomFloatinRange -2e+02 2e+02)) _z) (Math|Rotator|MakeRotator 0.0 0.0 (Math|Random|RandomFloatinRange 0.0 359.0)) (.scale _returnvalue)) "AdjustIfPossibleButDontSpawnIfColliding" 0 0)))

(fn ConstructionScript)